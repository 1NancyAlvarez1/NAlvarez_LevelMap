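; BP_Locker is a locker the player can hide in and leave with the Hide input.
; Box overlap with the first-person character toggles its prompt widget flag, locker input and a Gate, and stores the character reference on entry.
; Each press runs ToggleHide, flipping the character's visibility and collision and blending the camera between locker and character.
; The same press plays a timeline that rotates the door between closed and open angles.
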(event `InputAction|Hide`
  (params (Key :type "Key Structure"))
  ; In/Out Locker
  (:`Pressed`
    (`/Engine/EditorBlueprintResources/StandardMacros.Gate` false :!label _label
      (:`Exit`
        (`|ExecutionSequence`
          (:`then_0`
            (`self.ToggleHide`)
            (`KismetSystemLibrary.Delay` 0.2)
            (`self.EnableInput` (`GameplayStatics.GetPlayerController` 0) :!label _label_2)
            (goto _label :!via `Open`))
          (:`then_1`
            (bind (_direction _doortrack) (`Timeline|OpenCloseDoor_T` :!via `PlayFromStart`)
              (:`Update`
                (`SceneComponent.K2_SetRelativeRotation` (`self.SM_Locker_Door`) (`KismetMathLibrary.MakeRotator` 0.0 0.0 (`KismetMathLibrary.Lerp` (`self.Close Angle`) (`self.Open Angle`) _doortrack)) false false)))))))))

(event `self.Box.OnComponentBeginOverlap`
  (params (OverlappedComponent :type "PrimitiveComponent Object Reference") (OtherActor :type "Actor Object Reference") (OtherComp :type "PrimitiveComponent Object Reference") (OtherBodyIndex :type Integer) (bFromSweep :type Boolean) (SweepResult :type "HitResult Structure (by ref)"))
  ; In/Out Locker
  (bind _asbp_first_person_character (cast `/Game/FirstPerson/Blueprints/BP_FirstPersonCharacter` OtherActor))
  (set `/Game/FirstPerson/Blueprints/BP_FirstPersonCharacter.WIdgetVisible?` true _asbp_first_person_character)
  (bind _asbp_first_person_character_2 (cast `/Game/FirstPerson/Blueprints/BP_FirstPersonCharacter` OtherActor))
  (set `self.Char Ref` _asbp_first_person_character_2)
  (goto _label_2))

(event `self.Box.OnComponentEndOverlap`
  (params (OverlappedComponent :type "PrimitiveComponent Object Reference") (OtherActor :type "Actor Object Reference") (OtherComp :type "PrimitiveComponent Object Reference") (OtherBodyIndex :type Integer))
  ; In/Out Locker
  (bind _asbp_first_person_character (cast `/Game/FirstPerson/Blueprints/BP_FirstPersonCharacter` OtherActor))
  (set `/Game/FirstPerson/Blueprints/BP_FirstPersonCharacter.WIdgetVisible?` false _asbp_first_person_character)
  (`self.DisableInput` (`GameplayStatics.GetPlayerController` 0))
  (goto _label :!via `Close`))

(fn `ToggleHide`
  (bind _returnvalue (`GameplayStatics.GetPlayerController` 0))
  (bind _char_ref (`self.Char Ref`))
  (if (`self.IsHiding?`)
    (set `self.IsHiding?` false)
    (`self.SetActorHiddenInGame` _char_ref false)
    (`self.SetActorEnableCollision` _char_ref true)
    (`PlayerController.SetViewTargetWithBlend` _returnvalue _char_ref 2.0 "VTBlend_Linear" 0.0 false)
    (else
      (set `self.IsHiding?` true)
      (`self.SetActorHiddenInGame` _char_ref true)
      (`self.SetActorEnableCollision` _char_ref false)
      (`PlayerController.SetViewTargetWithBlend` _returnvalue self 0.8 "VTBlend_Linear" 0.0 false))))

(fn `UserConstructionScript`)